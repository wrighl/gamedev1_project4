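; Blueprint that creates the TextWidget text UI and forwards keyboard input to it.
; On BeginPlay it creates the widget, stores it as TextUI and adds it to the viewport.
; Enter, W and S trigger the widget's menu select, move up and move down functions, each only while the widget's Display flag is set.
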(event EventBeginPlay
  (bind _returnvalue (UserInterface|CreateWidget "/Game/TextWidget.TextWidget_C"))
  (bind _output_get (Variables|Default|SetTextUI _returnvalue))
  (UserInterface|Viewport|AddtoViewport _output_get 0))

(event EventTick
  (params (DeltaSeconds :type Float%20%28single-precision%29)))

(event Input|KeyboardEvents|Enter
  (params (Key :type Key%20Structure))
  (bind _textui (Variables|Default|GetTextUI))
  (:Pressed
    (if (Variables|/Game/TextWidget.TextWidget_C|GetDisplay _textui)
      (Default|MenuSelect _textui))))

(event Input|KeyboardEvents|W
  (params (Key :type Key%20Structure))
  (bind _textui (Variables|Default|GetTextUI))
  (:Pressed
    (if (Variables|/Game/TextWidget.TextWidget_C|GetDisplay _textui)
      (Default|MenuMoveUp _textui))))

(event Input|KeyboardEvents|S
  (params (Key :type Key%20Structure))
  (bind _textui (Variables|Default|GetTextUI))
  (:Pressed
    (if (Variables|/Game/TextWidget.TextWidget_C|GetDisplay _textui)
      (Default|MenuMoveDown _textui))))

(fn ConstructionScript)